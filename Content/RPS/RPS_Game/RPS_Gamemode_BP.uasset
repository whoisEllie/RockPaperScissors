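; Game mode for a Rock-Paper-Scissors game against a random AI, played until either side reaches three wins, then quits.
; A looping timer steps the widget through countdown prompts, then clears itself and resolves the round.
; Nested switches compare both choices, update score and prompt, and restart after a delay.
; Player button choices are stored and trigger the matching animation on the first BP_Hands actor found.
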(event Custom|StartGame
  (params (WidgetRef :type RPS%20HUD%20WBP%20Object%20Reference))
  (Variables|Default|SetWidget%20Ref WidgetRef)
  (bind _returnvalue (Utilities|Time|SetTimerbyEvent (delegate Custom|TextUpdate) 1.0 true 1.5))
  (Variables|Default|SetRoundStartTimer _returnvalue))

(event Custom|TextUpdate
  (Default|UpdatePrompt (Variables|Default|GetWidget%20Ref) (Utilities|Array|Get(acopy) (Variables|Default|GetNew%20Text) (Variables|Default|GetCurrentTextSelection)))
  (bind _result (Math|Integer|IncrementInt (Variables|Default|GetCurrentTextSelection))
    (:%20%20
      (if (> _result 4)
        (Variables|Default|SetCurrentTextSelection 0)
        (Utilities|Time|ClearandInvalidateTimerbyHandle (Variables|Default|GetRoundStartTimer))
        (CallFunction|CalculateResult)))))

(event Custom|CalculateResult
  (bind _widget_ref (Variables|Default|GetWidget%20Ref))
  (bind _widget_ref_2 (Variables|Default|GetWidget%20Ref))
  (bind _output_get (Variables|Default|SetAiChoice (Utilities|Enum|ByteToEnumEChoices (Math|Conversions|ToByte(Integer) (Math|Random|RandomIntegerinRange 0 2)))))
  (Default|UpdateAIChoice (Variables|Default|GetWidget%20Ref) _output_get)
  (switch Utilities|FlowControl|Switch|SwitchonEChoices (Variables|Default|GetPlayersChoice)
    (:NewEnumerator0
      (switch Utilities|FlowControl|Switch|SwitchonEChoices (Variables|Default|GetAiChoice)
        (:NewEnumerator0
          (Default|UpdatePrompt _widget_ref_2 "Draw" :!label _label)
          (Utilities|FlowControl|Delay 1.5 :!label _label_2)
          (CallFunction|NewRound)
          (Default|ClearAIChoice _widget_ref))
        (:NewEnumerator1
          (Default|UpdatePrompt _widget_ref_2 "Lose" :!label _label_3)
          (bind _result (Math|Integer|IncrementInt (Variables|Default|GetAiScore))
            (:%20%20
              (if (>= _result 3)
                (Default|UpdatePrompt _widget_ref "You Lost!")
                (Utilities|FlowControl|Delay 3.0 :!label _label_4)
                (Game|QuitGame 0 "Quit" false)
                (else
                  (goto _label_2))))))
        (:NewEnumerator2
          (Default|UpdatePrompt _widget_ref_2 "Win" :!label _label_5)
          (bind _result_2 (Math|Integer|IncrementInt (Variables|Default|GetPlayerScore))
            (:%20%20
              (if (>= _result_2 3)
                (Default|UpdatePrompt _widget_ref "You Win!")
                (goto _label_4)
                (else
                  (goto _label_2))))))))
    (:NewEnumerator1
      (switch Utilities|FlowControl|Switch|SwitchonEChoices (Variables|Default|GetAiChoice)
        (:NewEnumerator0
          (goto _label_5))
        (:NewEnumerator1
          (goto _label))
        (:NewEnumerator2
          (goto _label_3))))
    (:NewEnumerator2
      (switch Utilities|FlowControl|Switch|SwitchonEChoices (Variables|Default|GetAiChoice)
        (:NewEnumerator0
          (goto _label_3))
        (:NewEnumerator1
          (goto _label_5))
        (:NewEnumerator2
          (goto _label))))))

(event Custom|PlayerChoice
  (params (PlayerButton :type EChoices%20Enum :default "NewEnumerator0"))
  (bind _output_get (Variables|Default|SetPlayersChoice PlayerButton))
  (bind _outactors (Actor|GetAllActorsOfClass "/Game/RPS/RPS_Assets/BP_Hands.BP_Hands_C"))
  (switch Utilities|FlowControl|Switch|SwitchonEChoices _output_get
    (:NewEnumerator0
      (Default|PlayRock (Utilities|Array|Get(acopy) _outactors)))
    (:NewEnumerator1
      (Default|PlayPaper (Utilities|Array|Get(acopy) _outactors)))
    (:NewEnumerator2
      (Default|PlayScissors (Utilities|Array|Get(acopy) _outactors)))))

(event Custom|NewRound
  (bind _returnvalue (Utilities|Time|SetTimerbyEvent (delegate Custom|TextUpdate) 1.0 true 1.5))
  (Variables|Default|SetRoundStartTimer _returnvalue))

(event Custom|UpdateWidget
  (params (WidgetRef :type RPS%20HUD%20WBP%20Object%20Reference))
  (Variables|Default|SetWidget%20Ref WidgetRef)
  (CallFunction|TextUpdate))

(fn ConstructionScript)